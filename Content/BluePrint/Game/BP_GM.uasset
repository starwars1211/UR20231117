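; Game manager Blueprint for a timed target-hunting round, won by killing every BP_Sphere before the countdown expires.
; BeginPlay restores the target count from the GameInstance, counts the spheres and binds their OnDied events to CountTarget, which writes the count back.
; Tick runs the timer, and a DoOnce-guarded EndGame pauses play, reveals WG_GameUI's victory or failure panel and shows the cursor.
; Widget creation and best-time saving sit in unconnected nodes.
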(event Custom|EndGame
  (params (isVictory :type Boolean))
  (Utilities|FlowControl|DoOnce false
    (:Completed
      (Game|SetGamePaused true)
      (if isVictory
        (bind _foundwidgets (Widget|GetAllWidgetsOfClass "/Game/BluePrint/UI_Widget/WG_GameUI.WG_GameUI_C" true))
        (for _array_element _foundwidgets
          (Utilities|IsValid "/Game/BluePrint/UI_Widget/WG_GameUI.WG_GameUI"
            (:Is%20Valid
              (Variables|/Script/UMG.Widget|SetVisibility (Variables|/Game/BluePrint/UI_Widget/WG_GameUI.WG_GameUI_C|GetEndVictory _array_element) "Visible")
              (CallFunction|EndMoniter))))
        (else
          (bind _foundwidgets_2 (Widget|GetAllWidgetsOfClass "/Game/BluePrint/UI_Widget/WG_GameUI.WG_GameUI_C" true))
          (for _array_element_2 _foundwidgets_2
            (Utilities|IsValid "/Game/BluePrint/UI_Widget/WG_GameUI.WG_GameUI"
              (:Is%20Valid
                (Variables|/Script/UMG.Widget|SetVisibility (Variables|/Game/BluePrint/UI_Widget/WG_GameUI.WG_GameUI_C|GetEndFailed _array_element_2) "Visible")
                (CallFunction|EndMoniter)))))))))

(event Custom|EndMoniter
  (bind _foundwidgets (Widget|GetAllWidgetsOfClass "/Game/BluePrint/UI_Widget/WG_GameUI.WG_GameUI_C" true))
  (for _array_element _foundwidgets
    (Utilities|IsValid "/Game/BluePrint/UI_Widget/WG_GameUI.WG_GameUI"
      (:Is%20Valid
        (Variables|/Script/UMG.Widget|SetVisibility (Variables|/Game/BluePrint/UI_Widget/WG_GameUI.WG_GameUI_C|GetEndVertical _array_element) "Visible")
        (Variables|/Script/Engine.PlayerController|SetbShowMouseCursor (Game|GetPlayerController 0) true)))))

(event Custom|OnDied_Event
  ;[1 1 1 1 25] 타겟카운트를 가져온다 타임을 맥스로 설정하고스피어타겟을 맥스로 Set온다이이벤
  (CallFunction|CountTarget))

(event EventBeginPlay
  ;[1 1 1 1 25] 타겟카운트를 가져온다 타임을 맥스로 설정하고스피어타겟을 맥스로 Set온다이이벤
  (Utilities|FlowControl|Sequence
    (:then_0
      (bind _spherecount (Class|BPInterface|GetCount(Message) (Game|GetGameInstance)))
      (Variables|Default|SetTargetCount _spherecount))
    (:then_1
      (Variables|Default|SetTime (Variables|Default|GetMaxTime))
      (bind _outactors (Actor|GetAllActorsOfClass "/Game/BluePrint/Actor/BP_Sphere.BP_Sphere_C"))
      (Variables|Default|SetMaxTarget (Utilities|Array|Length _outactors))
      (for _array_element _outactors
        (EventDispatchers|BindEventtoOnDied _array_element (delegate Custom|OnDied_Event))))))

(event EventTick
  (params (DeltaSeconds :type Float%20%28single-precision%29))
  ;[1 1 1] 시간이 다되면 게임이 끝나는 노드
  (if true
    (bind _output_get (Variables|Default|SetTime (- (Variables|Default|GetTime) DeltaSeconds)))
    (if (<= _output_get 0.0)
      (CallFunction|EndGame false))))

(fn ConstructionScript)

(fn CountTarget
  (Utilities|FlowControl|Sequence
    (:then_0
      (bind _result (Math|Integer|IncrementInt (Variables|Default|GetTargetCount))
        (:%20%20
          (if (>= _result (Variables|Default|GetMaxTarget))
            (CallFunction|EndGame true)))))
    (:then_1
      (Class|BPInterface|SetCount(Message) (Game|GetGameInstance) (Variables|Default|GetTargetCount))
      (Utilities|Casting|CastToBP_GI (Game|GetGameInstance)))))