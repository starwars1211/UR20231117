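; Player pawn that fires hitscan shots on left mouse click, with switchable Single and Multy fire modes.
; Shot line-traces forward from the camera on the Visibility channel and applies damage to the hit actor.
; Multy presses also set a short non-looping timer, cleared on release.
; ChangeGun sets the mode; for Multy, a 10-second retriggerable delay clears that timer but reassigns Multy rather than reverting to Single.
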(event Custom|Shot
  (bind _returnvalue (Game|GetPlayerCameraManager 0))
  (bind _returnvalue_2 (Transformation|GetActorLocation _returnvalue))
  ;[1 1 1 1 25] 총 나가는 것을 표현한 노드(카메라가 액터를 벡터값으로 표현
  (bind (_outhit _returnvalue_3) (Collision|LineTraceByChannel _returnvalue_2 (+ _returnvalue_2 (* (Math|Vector|GetForwardVector (Transformation|GetActorRotation _returnvalue)) 1e+04)) "TraceTypeQuery1" false 0 "None"))
  (if _returnvalue_3
    (Game|Damage|ApplyDamage (.HitActor (Collision|BreakHitResult _outhit)) 1.0 0 0)))

(event Custom|ChangeGun
  (params (NewParam :type Enum_GunChange%20Enum :default "NewEnumerator0"))
  ;[1 1 1 1 25] 연사로 10초동안 바꾼다는 노드
  (Variables|Default|SetSwitch_ShotMode NewParam)
  (switch Utilities|FlowControl|Switch|SwitchonEnum_GunChange NewParam
    (:NewEnumerator2
      (Utilities|FlowControl|RetriggerableDelay 1e+01)
      (Variables|Default|SetSwitch_ShotMode "NewEnumerator2")
      (Utilities|Time|ClearandInvalidateTimerbyHandle (Variables|Default|GetMultyShotHandle)))))

(event EventBeginPlay)

(event Collision|EventActorBeginOverlap
  (params (OtherActor :type Actor%20Object%20Reference)))

(event EventTick
  (params (DeltaSeconds :type Float%20%28single-precision%29)))

(event Input|MouseEvents|LeftMouseButton
  (params (Key :type Key%20Structure :default "None"))
  (bind _switch_shotmode (Variables|Default|GetSwitch_ShotMode))
  ;[1 1 1 1 25] 싱글일땐 한번만 실행 연사일땐 멀티샷핸들일때 동안0.005마다
  (:Pressed
    (switch Utilities|FlowControl|Switch|SwitchonEnum_GunChange _switch_shotmode
      (:NewEnumerator1
        (CallFunction|Shot))
      (:NewEnumerator2
        (bind _returnvalue (Utilities|Time|SetTimerbyEvent 0 0.005))
        (Variables|Default|SetMultyShotHandle _returnvalue)
        (CallFunction|Shot))))
  (:Released
    (switch Utilities|FlowControl|Switch|SwitchonEnum_GunChange _switch_shotmode
      (:NewEnumerator2
        (Utilities|Time|ClearandInvalidateTimerbyHandle (Variables|Default|GetMultyShotHandle))))))

(fn ConstructionScript)