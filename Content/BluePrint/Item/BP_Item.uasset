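; BP_Item is a pickup actor that plays a sound and destroys itself when anything overlaps its sphere.
; The overlap calls ItemOverlap for the sound, then DestroyActor, then TimeUp, which is empty here.
; BeginPlay caches the BP_GM game mode, but the clamped logic that adds time to it is disconnected and never runs.
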(event OnComponentBeginOverlap(Sphere)
  (params (OverlappedComponent :type Primitive%20Component%20Object%20Reference) (OtherActor :type Actor%20Object%20Reference) (OtherComp :type Primitive%20Component%20Object%20Reference) (OtherBodyIndex :type Integer) (bFromSweep :type Boolean) (SweepResult :type Hit%20Result%20Structure%20%28by%20ref%29))
  (CallFunction|ItemOverlap)
  (Actor|DestroyActor)
  (CallFunction|TimeUp))

(event Custom|ItemOverlap
  (Audio|PlaySound2D (Variables|Default|GetSound) 1.0 1.0 0.0 0 0))

(event Custom|TimeUp)

(event EventBeginPlay
  (bind _asbp_gm (Utilities|Casting|CastToBP_GM (Game|GetGameMode)))
  (Variables|Default|SetBP_GMReference _asbp_gm))

(event Collision|EventActorBeginOverlap
  (params (OtherActor :type Actor%20Object%20Reference)))

(event EventTick
  (params (DeltaSeconds :type Float%20%28single-precision%29)))

(fn ConstructionScript)