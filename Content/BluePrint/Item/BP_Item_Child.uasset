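; BP_Item_Child is a pickup item, derived from a parent item Blueprint, that raises the game mode's target count.
; BeginPlay caches BP_GM without calling the parent's BeginPlay.
; Any Sphere overlap, with no filter on the other actor, runs the parent's ItemOverlap, destroys the actor, then calls its own ItemOverlap.
; That event adds a fixed bonus to TargetCount and clamps it to a bounded range.
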(event OnComponentBeginOverlap(Sphere)
  (params (OverlappedComponent :type Primitive%20Component%20Object%20Reference) (OtherActor :type Actor%20Object%20Reference) (OtherComp :type Primitive%20Component%20Object%20Reference) (OtherBodyIndex :type Integer) (bFromSweep :type Boolean) (SweepResult :type Hit%20Result%20Structure%20%28by%20ref%29))
  (|CallParentFunction)
  (Actor|DestroyActor)
  (CallFunction|ItemOverlap))

(event EventBeginPlay
  (bind _asbp_gm (Utilities|Casting|CastToBP_GM (Game|GetGameMode)))
  (Variables|Default|SetAs%20BP%20GM _asbp_gm))

(event Collision|EventActorBeginOverlap
  (params (OtherActor :type Actor%20Object%20Reference))
  (|CallParentFunction OtherActor) ; This node is disabled and will not be called.\nDrag off pins to build functionality.
)

(event EventTick
  (params (DeltaSeconds :type Float%20%28single-precision%29))
  (|CallParentFunction DeltaSeconds) ; This node is disabled and will not be called.\nDrag off pins to build functionality.
)

(event EventItemOverlap
  (Variables|/Game/BluePrint/Game/BP_GM.BP_GM_C|SetTargetCount (Variables|Default|GetAs%20BP%20GM) (Math|Integer|Clamp(Integer) (+ (Variables|/Game/BluePrint/Game/BP_GM.BP_GM_C|GetTargetCount (Variables|Default|GetAs%20BP%20GM)) 5) 1 10)))

(fn ConstructionScript
  (|CallParentFunction))